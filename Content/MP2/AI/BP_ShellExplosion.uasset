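; BP_ShellExplosion is a short-lived explosion actor, apparently from an AI shell, that damages and knocks back the player.
; On BeginPlay it spawns an explosion particle on its root and destroys itself after a brief delay.
; When its detection component overlaps the learning-kit player character, it launches them away from the blast origin, decrements their health, then also schedules self-destruction.
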(event `self.ReceiveBeginPlay`
  (`GameplayStatics.SpawnEmitterAttached` "/Game/StarterContent/Particles/P_Explosion.P_Explosion" (`self.DefaultSceneRoot`))
  (`KismetSystemLibrary.Delay` 0.5)
  (`self.K2_DestroyActor` :!label _label))

(event `self.ExplosionDetection.OnComponentBeginOverlap`
  (params (OverlappedComponent :type "PrimitiveComponent Object Reference") (OtherActor :type "Actor Object Reference") (OtherComp :type "PrimitiveComponent Object Reference") (OtherBodyIndex :type Integer) (bFromSweep :type Boolean) (SweepResult :type "HitResult Structure (by ref)"))
  (bind _asbp_learning_kit_player_character (cast `/Game/LearningKit_Games/Blueprints/PlayerCharacter/BP_LearningKit_PlayerCharacter` OtherActor))
  (`/Game/LearningKit_Games/Blueprints/PlayerCharacter/BP_LearningKit_PlayerCharacter.GetsLaunched` _asbp_learning_kit_player_character (`SceneComponent.K2_GetComponentLocation` (`self.DefaultSceneRoot`)) 1000.0)
  (`/Game/LearningKit_Games/Blueprints/PlayerCharacter/BP_LearningKit_PlayerCharacter.DecrementHealth` _asbp_learning_kit_player_character)
  (`KismetSystemLibrary.Delay` 0.5)
  (goto _label))

(fn `UserConstructionScript`)