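; BP_Mortar is a stationary enemy that periodically lobs shells and can be killed by a hit to its head.
; A looping timer calls ShootShell, which spawns a BP_MortarShell at Firepoint and gives it physics velocity toward a random nearby navigable point with fixed upward lift.
; Player overlap with the body hitbox launches and damages the player.
; Player overlap with the head hitbox awards score and destroys the mortar.
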(event `self.ReceiveBeginPlay`
  (`KismetSystemLibrary.K2_SetTimer` null "ShootShell" 3.0 true 3.0))

(event `self.Bodyhitbox.OnComponentBeginOverlap`
  (params (OverlappedComponent :type "PrimitiveComponent Object Reference") (OtherActor :type "Actor Object Reference") (OtherComp :type "PrimitiveComponent Object Reference") (OtherBodyIndex :type Integer) (bFromSweep :type Boolean) (SweepResult :type "HitResult Structure (by ref)"))
  ;[1 1 1] knockback on body hit
  (if (== OtherActor (`GameplayStatics.GetPlayerCharacter` 0))
    (bind _asbp_learning_kit_player_character (cast `/Game/LearningKit_Games/Blueprints/PlayerCharacter/BP_LearningKit_PlayerCharacter` OtherActor))
    (`/Game/LearningKit_Games/Blueprints/PlayerCharacter/BP_LearningKit_PlayerCharacter.GetsLaunched` _asbp_learning_kit_player_character (`self.K2_GetActorLocation`) (`self.KnockBackBelocity`))
    (`/Game/LearningKit_Games/Blueprints/PlayerCharacter/BP_LearningKit_PlayerCharacter.DecrementHealth` _asbp_learning_kit_player_character)))

(event `self.HeadHitbox.OnComponentBeginOverlap`
  (params (OverlappedComponent :type "PrimitiveComponent Object Reference") (OtherActor :type "Actor Object Reference") (OtherComp :type "PrimitiveComponent Object Reference") (OtherBodyIndex :type Integer) (bFromSweep :type Boolean) (SweepResult :type "HitResult Structure (by ref)"))
  ;[1 1 1] kill self on head hit
  (if (== OtherActor (`GameplayStatics.GetPlayerCharacter` 0))
    (bind _asbp_learning_kit_player_character (cast `/Game/LearningKit_Games/Blueprints/PlayerCharacter/BP_LearningKit_PlayerCharacter` OtherActor))
    (`/Game/LearningKit_Games/Blueprints/PlayerCharacter/BP_LearningKit_PlayerCharacter.IncrementScore` _asbp_learning_kit_player_character)
    (`self.K2_DestroyActor`)))

(fn `ShootShell`
  (bind (_returnvalue_location _returnvalue_rotation) (`KismetMathLibrary.BreakTransform` (`SceneComponent.K2_GetComponentToWorld` (`self.firepoint`))))
  (bind _returnvalue (`SceneComponent.K2_GetComponentLocation` (`self.firepoint`)))
  (bind (_returnvalue_x _returnvalue_y) (`KismetMathLibrary.BreakVector` (`KismetMathLibrary.GetDirectionUnitVector` _returnvalue (`NavigationSystemV1.K2_GetRandomLocationInNavigableRadius` _returnvalue 500.0 null null))))
  (bind _returnvalue_2 (`|SpawnActorFromClass` "/Game/MP2/AI/BP_MortarShell.BP_MortarShell_C" (`KismetMathLibrary.MakeTransform` _returnvalue_location _returnvalue_rotation) "Undefined" "OverrideRootScale" self null))
  (`PrimitiveComponent.SetPhysicsLinearVelocity` (`/Game/MP2/AI/BP_MortarShell.Sphere` _returnvalue_2) (`KismetMathLibrary.MakeVector` (* _returnvalue_x 800.0) (* _returnvalue_y 800.0) 750.0) false "None"))

(fn `UserConstructionScript`)