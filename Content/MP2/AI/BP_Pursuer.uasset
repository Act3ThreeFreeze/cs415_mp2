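; Enemy AI character that chases the player on sight and roams randomly otherwise, and can be defeated by hitting its head.
; PawnSensing starts the chase, while a retriggerable delay and Tick-driven delays clear the chase flags and pick random reachable roam points.
; Head overlap increments player score and destroys the enemy; body overlap launches the player and decrements health.
; A separate KnockBackPlayer function with launch and stun is not called here.
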(event `self.PawnSensing.OnSeePawn`
  (params (Pawn :type "Pawn Object Reference"))
  (bind _asbp_learning_kit_player_character (cast `/Game/LearningKit_Games/Blueprints/PlayerCharacter/BP_LearningKit_PlayerCharacter` Pawn))
  (`|ExecutionSequence`
    (:`then_0`
      (set `self.SeenPlayerRecently` true)
      (set `self.IsChasing` true)
      (`|AIMoveTo` self (0.0 0.0 0.0) _asbp_learning_kit_player_character))
    (:`then_1`
      (`KismetSystemLibrary.RetriggerableDelay` 0.6)
      (set `self.SeenPlayerRecently` false))))

(event `self.ReceiveTick`
  (params (DeltaSeconds :type "Float (single-precision)"))
  ;[1 1 1] AI Random Roam
  (`|ExecutionSequence`
    (:`then_0`
      (if (not (`self.SeenPlayerRecently`))
        (`KismetSystemLibrary.Delay` 0.4)
        (if (not (`self.SeenPlayerRecently`))
          (set `self.IsChasing` false))))
    (:`then_1`
      (if (not (`self.IsChasing`))
        (`KismetSystemLibrary.Delay` (`KismetMathLibrary.RandomFloatInRange` 1.5 2.5))
        (`|AIMoveTo` self (`NavigationSystemV1.K2_GetRandomReachablePointInRadius` (`self.K2_GetActorLocation`) 1000.0 null null) null)))))

(event `self.ReceiveBeginPlay`)

(event `self.HeadHitbox.OnComponentBeginOverlap`
  (params (OverlappedComponent :type "PrimitiveComponent Object Reference") (OtherActor :type "Actor Object Reference") (OtherComp :type "PrimitiveComponent Object Reference") (OtherBodyIndex :type Integer) (bFromSweep :type Boolean) (SweepResult :type "HitResult Structure (by ref)"))
  (bind _returnvalue (`GameplayStatics.GetPlayerCharacter` 0))
  ;[1 1 1] player hit me head!
  (if (== OtherActor _returnvalue)
    (bind _asbp_learning_kit_player_character (cast `/Game/LearningKit_Games/Blueprints/PlayerCharacter/BP_LearningKit_PlayerCharacter` _returnvalue))
    (`/Game/LearningKit_Games/Blueprints/PlayerCharacter/BP_LearningKit_PlayerCharacter.IncrementScore` _asbp_learning_kit_player_character)
    (`self.K2_DestroyActor`)))

(event `self.BodyHitbox.OnComponentBeginOverlap`
  (params (OverlappedComponent :type "PrimitiveComponent Object Reference") (OtherActor :type "Actor Object Reference") (OtherComp :type "PrimitiveComponent Object Reference") (OtherBodyIndex :type Integer) (bFromSweep :type Boolean) (SweepResult :type "HitResult Structure (by ref)"))
  (bind _returnvalue (`GameplayStatics.GetPlayerCharacter` 0))
  ;[1 1 1] KnockPlayerBack
  (if (== OtherActor _returnvalue)
    (bind _asbp_learning_kit_player_character (cast `/Game/LearningKit_Games/Blueprints/PlayerCharacter/BP_LearningKit_PlayerCharacter` _returnvalue))
    (`KismetSystemLibrary.PrintString` "Enemy body hit")
    (`/Game/LearningKit_Games/Blueprints/PlayerCharacter/BP_LearningKit_PlayerCharacter.GetsLaunched` _asbp_learning_kit_player_character (`self.K2_GetActorLocation`) (`self.KnockBackVelocity`))
    (`/Game/LearningKit_Games/Blueprints/PlayerCharacter/BP_LearningKit_PlayerCharacter.DecrementHealth` _asbp_learning_kit_player_character)))

(fn `KnockBackPlayer`
  (params (NewParam :type "/Game/LearningKit_Games/Blueprints/PlayerCharacter/BP_LearningKit_PlayerCharacter Object Reference"))
  (bind (_returnvalue_x _returnvalue_y _returnvalue_z) (`KismetMathLibrary.BreakVector` (`KismetMathLibrary.GetDirectionUnitVector` (`SceneComponent.K2_GetComponentLocation` (`self.CapsuleComponent`)) (`self.K2_GetActorLocation`))))
  (`self.LaunchCharacter` NewParam (* (`KismetMathLibrary.MakeVector` _returnvalue_x _returnvalue_y (+ _returnvalue_z 0.4)) (`self.KnockBackVelocity`)) false false)
  (`/Game/LearningKit_Games/Blueprints/PlayerCharacter/BP_LearningKit_PlayerCharacter.GettingStunned` NewParam))

(fn `UserConstructionScript`)